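; First-person shooter player character Blueprint handling movement, look, jumping, shooting and damage.
; On BeginPlay it creates the HUD and attaches a spawned weapon to a mesh socket.
; Input drives looping automatic fire at the weapon's rate, reloading that blocks firing and aiming, and aim-down-sights by camera switching.
; Projectile overlaps reduce health, more on the head hitbox; Tick checks health and destroys character and weapon after a delay at zero.
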(event `self.ReceiveTick`
  (params (DeltaSeconds :type "Float (single-precision)"))
  ;[0 1 0.7656] Event Tick
  (bind _output_get (`self.CheckLife`))
  (if _output_get
    (`KismetSystemLibrary.Delay` 2.0)
    (`self.K2_DestroyActor`)
    (`self.K2_DestroyActor` (`self.EquipedWeapon`))))

(event `InputAxis|Turn`
  (params (AxisValue :type "Float (single-precision)"))
  ;[1 0.9015 0] Gestion des déplacement
  (`self.AddControllerYawInput` (* AxisValue (`self.BaseTurnRate`) (`GameplayStatics.GetWorldDeltaSeconds`))))

(event `self.ReceiveBeginPlay`
  ;[0 1 1] Begin Play Event
  (`self.CreateHUD`)
  (`self.SpawnWeapon`))

(event `InputAxis|LookUp`
  (params (AxisValue :type "Float (single-precision)"))
  ;[1 0.9015 0] Gestion des déplacement
  (`self.AddControllerPitchInput` (* AxisValue (`self.BaseLookUpRate`) (`GameplayStatics.GetWorldDeltaSeconds`))))

(event `InputAction|Reload`
  (params (Key :type "Key Structure"))
  ;[1 0 0] Weapon system
  (:`Pressed`
    (set `self.isAiming` false)
    (bind (_output_get _output_get1) (`/Game/Blueprints/Weapons/Weapon_Base.Reload` (`self.EquipedWeapon`)))
    (if (or _output_get _output_get1)
      (`KismetSystemLibrary.Delay` 2.167)
      (set `self.isReloading` false))))

(event `InputAction|Jump` :overrideparent false
  (params (Key :type "Key Structure"))
  ;[1 0.9015 0] Gestion des déplacement
  (:`Pressed`
    (`self.Jump`))
  (:`Released`
    (`self.StopJumping`)))

(event `InputAction|Aiming`
  (params (Key :type "Key Structure"))
  ;[1 0 0] Weapon system
  (:`Pressed`
    (if (not (`self.isReloading`))
      (`self.Scope`)
      (set `self.isAiming` true)))
  (:`Released`
    (`self.Unscope`)
    (set `self.isAiming` false)))

(event `InputAxis|Turn` :overrideparent false
  (params (AxisValue :type "Float (single-precision)"))
  ;[1 0.9015 0] Gestion des déplacement
  (`self.AddControllerYawInput` AxisValue))

(event `InputAction|PrimaryFire`
  (params (Key :type "Key Structure"))
  (bind _equipedweapon (`self.EquipedWeapon`))
  ;[1 0 0] Weapon system
  (:`Pressed`
    (if (not (`self.isReloading`))
      (if (> (`/Game/Blueprints/Weapons/Weapon_Base.Ammo` (`self.EquipedWeapon`)) 0) :!label _label
        (set `self.isFiring` true)
        (`/Game/Blueprints/Weapons/Weapon_Base.Fire` _equipedweapon)
        (`KismetSystemLibrary.Delay` (`/Game/Blueprints/Weapons/Weapon_Base.FireRate` _equipedweapon))
        (if (`self.isFiring`)
          (goto _label)))))
  (:`Released`
    (set `self.isFiring` false)))

(event `InputAxis|LookUp` :overrideparent false
  (params (AxisValue :type "Float (single-precision)"))
  ;[1 0.9015 0] Gestion des déplacement
  (`self.AddControllerPitchInput` AxisValue))

(event `InputAxis|MoveForward` :overrideparent false
  (params (AxisValue :type "Float (single-precision)"))
  ;[1 0.9015 0] Gestion des déplacement
  (`self.AddMovementInput` (`KismetMathLibrary.GetForwardVector` (`KismetMathLibrary.MakeRotator` 0.0 0.0 (.yaw (`self.GetControlRotation`)))) AxisValue))

(event `InputAxis|MoveRight` :overrideparent false
  (params (AxisValue :type "Float (single-precision)"))
  ;[1 0.9015 0] Gestion des déplacement
  (`self.AddMovementInput` (`KismetMathLibrary.GetRightVector` (`KismetMathLibrary.MakeRotator` 0.0 0.0 (.yaw (`self.GetControlRotation`)))) AxisValue))

(event `self.HitBoxHead.OnComponentBeginOverlap`
  (params (OverlappedComponent :type "PrimitiveComponent Object Reference") (OtherActor :type "Actor Object Reference") (OtherComp :type "PrimitiveComponent Object Reference") (OtherBodyIndex :type Integer) (bFromSweep :type Boolean) (SweepResult :type "HitResult Structure (by ref)"))
  ;[0.3594 1 0] Gestion de la prise des dégats
  (cast `/Game/Blueprints/Weapons/Projectiles/Projectile_Base` OtherActor)
  (set `self.Health` (- (`self.Health`) 0.8))
  (`KismetSystemLibrary.PrintString` "headshot"))

(event `self.Capsule.OnComponentBeginOverlap`
  (params (OverlappedComponent :type "PrimitiveComponent Object Reference") (OtherActor :type "Actor Object Reference") (OtherComp :type "PrimitiveComponent Object Reference") (OtherBodyIndex :type Integer) (bFromSweep :type Boolean) (SweepResult :type "HitResult Structure (by ref)"))
  ;[0.3594 1 0] Gestion de la prise des dégats
  (cast `/Game/Blueprints/Weapons/Projectiles/Projectile_Base` OtherActor)
  (set `self.Health` (- (`self.Health`) 0.2))
  (`KismetSystemLibrary.PrintString` "Bodyshot"))

(fn `CheckLife`
  (returns (Output_Get :type Boolean))
  (if (<= (`self.Health`) 0.0)
    (bind _output_get (set `self.isDead` true))
    (return _output_get)))

(fn `CreateHUD`
  (bind _returnvalue (`|CreateWidget` "/Game/Blueprints/HUD/HUD_FPS.HUD_FPS_C"))
  (`UserWidget.AddToViewport` _returnvalue 0))

(fn `Diying`)

(fn `OnRep_Score`)

(fn `Scope`
  (`ActorComponent.Deactivate` (`self.Camera`))
  (`ActorComponent.Activate` (`self.AimCamera`) false))

(fn `SpawnWeapon`
  (bind _returnvalue (`|SpawnActorFromClass` "/Game/Blueprints/Weapons/Weapon_Base.Weapon_Base_C" (`KismetMathLibrary.MakeTransform` (0.0 0.0 0.0)) "Undefined" "OverrideRootScale" null null))
  (bind _output_get (set `self.EquipedWeapon` _returnvalue))
  (`self.K2_AttachToComponent` _output_get (`self.Mesh`) "Weapon_Socket" "SnapToTarget" "SnapToTarget" "SnapToTarget" true))

(fn `Unscope`
  (`ActorComponent.Deactivate` (`self.AimCamera`))
  (`ActorComponent.Activate` (`self.Camera`) false))

(fn `UserConstructionScript`)