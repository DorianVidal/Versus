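; Base weapon with hitscan firing and reloading, tied to player character 0.
; Fire traces from the aim or normal camera with persistent debug lines, spends ammo unchecked and spawns a muzzle flash.
; A hit Player_BP loses health and is destroyed at zero, otherwise an explosion effect spawns at impact.
; Reload refills the clip from MaxAmmo and flags the player as reloading; an alternative projectile path is left unconnected.
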(event `Fire`
  (bind _asplayer_bp (cast `/Game/Blueprints/Player/Player_BP` (`GameplayStatics.GetPlayerCharacter` 0)))
  (if (`/Game/Blueprints/Player/Player_BP.isAiming` _asplayer_bp)
    (bind _aimcamera (`/Game/Blueprints/Player/Player_BP.AimCamera` _asplayer_bp))
    (bind _returnvalue (`SceneComponent.K2_GetComponentLocation` _aimcamera))
    (bind _outhit (`KismetSystemLibrary.LineTraceSingle` :`Start` _returnvalue :`End` (+ _returnvalue (* (`KismetMathLibrary.GetForwardVector` (`SceneComponent.K2_GetComponentRotation` _aimcamera)) 1500)) :`TraceChannel` "TraceTypeQuery1" :`DrawDebugType` "Persistent"))
    (set `self.Ammo` (- (`self.Ammo`) 1))
    (bind _asplayer_bp_2 (cast `/Game/Blueprints/Player/Player_BP` (`GameplayStatics.GetPlayerCharacter` 0)))
    (bind _skeletalmesh (`/Game/Blueprints/Weapons/Weapon_Base.SkeletalMesh` (`/Game/Blueprints/Player/Player_BP.EquipedWeapon` _asplayer_bp_2)))
    (bind _returnvalue_2 (`GameplayStatics.SpawnEmitterAtLocation` "/Game/3D_(anim_meshes)/InfinityBladeEffects/Effects/FX_Mobile/Fire/combat/P_FireBall_Strong_MuzzFlash_01.P_FireBall_Strong_MuzzFlash_01" (`SceneComponent.GetSocketLocation` _skeletalmesh "Muzzle") (`SceneComponent.GetSocketRotation` _skeletalmesh "Muzzle")))
    (`SceneComponent.SetWorldScale3D` _returnvalue_2 (0.2 0.2 0.2))
    (bind (_bblockinghit _binitialoverlap _time _distance _location _impactpoint _normal _impactnormal _physmat _hitactor) (`GameplayStatics.BreakHitResult` _outhit))
    (bind _asplayer_bp_3 (cast `/Game/Blueprints/Player/Player_BP` _hitactor))
    (bind _output_get (set `/Game/Blueprints/Player/Player_BP.Health` (- (`/Game/Blueprints/Player/Player_BP.Health` _asplayer_bp_3) 0.5) _asplayer_bp_3))
    (if (<= _output_get 0.0)
      (`self.K2_DestroyActor` _asplayer_bp_3)
      (else
        (`GameplayStatics.SpawnEmitterAtLocation` "/Game/3D_(anim_meshes)/InfinityBladeEffects/Effects/FX_Cines/cinema03/P_CIN_IB_Explosion.P_CIN_IB_Explosion" _location)))
    (else
      (bind _camera (`/Game/Blueprints/Player/Player_BP.Camera` _asplayer_bp))
      (bind _returnvalue_3 (`SceneComponent.K2_GetComponentLocation` _camera))
      (bind _outhit_2 (`KismetSystemLibrary.LineTraceSingle` :`Start` _returnvalue_3 :`End` (+ _returnvalue_3 (* (`KismetMathLibrary.GetForwardVector` (`SceneComponent.K2_GetComponentRotation` _camera)) 1500)) :`TraceChannel` "TraceTypeQuery1" :`DrawDebugType` "Persistent"))
      (set `self.Ammo` (- (`self.Ammo`) 1))
      (bind _asplayer_bp_4 (cast `/Game/Blueprints/Player/Player_BP` (`GameplayStatics.GetPlayerCharacter` 0)))
      (bind _skeletalmesh_2 (`/Game/Blueprints/Weapons/Weapon_Base.SkeletalMesh` (`/Game/Blueprints/Player/Player_BP.EquipedWeapon` _asplayer_bp_4)))
      (bind _returnvalue_4 (`GameplayStatics.SpawnEmitterAtLocation` "/Game/3D_(anim_meshes)/InfinityBladeEffects/Effects/FX_Mobile/Fire/combat/P_FireBall_Strong_MuzzFlash_01.P_FireBall_Strong_MuzzFlash_01" (`SceneComponent.GetSocketLocation` _skeletalmesh_2 "Muzzle") (`SceneComponent.GetSocketRotation` _skeletalmesh_2 "Muzzle")))
      (`SceneComponent.SetWorldScale3D` _returnvalue_4 (0.2 0.2 0.2))
      (bind (_bblockinghit_2 _binitialoverlap_2 _time_2 _distance_2 _location_2 _impactpoint_2 _normal_2 _impactnormal_2 _physmat_2 _hitactor_2) (`GameplayStatics.BreakHitResult` _outhit_2))
      (bind _asplayer_bp_5 (cast `/Game/Blueprints/Player/Player_BP` _hitactor_2))
      (bind _output_get_2 (set `/Game/Blueprints/Player/Player_BP.Health` (- (`/Game/Blueprints/Player/Player_BP.Health` _asplayer_bp_5) 0.5) _asplayer_bp_5))
      (if (<= _output_get_2 0.0)
        (`self.K2_DestroyActor` _asplayer_bp_5)
        (else
          (`GameplayStatics.SpawnEmitterAtLocation` "/Game/3D_(anim_meshes)/InfinityBladeEffects/Effects/FX_Cines/cinema03/P_CIN_IB_Explosion.P_CIN_IB_Explosion" _location_2))))))

(fn `Reload`
  (returns (Output_Get :type Boolean) (Output_Get1 :type Boolean))
  (if (not (== (`self.Ammo`) (`self.ClipSize`)))
    (if (> (`self.MaxAmmo`) (`self.ClipSize`))
      (set `self.Ammo` (`self.ClipSize`))
      (set `self.MaxAmmo` (- (`self.MaxAmmo`) (`self.ClipSize`)))
      (bind _asplayer_bp (cast `/Game/Blueprints/Player/Player_BP` (`GameplayStatics.GetPlayerCharacter` 0)))
      (bind _output_get (set `/Game/Blueprints/Player/Player_BP.isReloading` true _asplayer_bp))
      (else
        (set `self.Ammo` (`self.MaxAmmo`))
        (set `self.MaxAmmo` 0)
        (bind _asplayer_bp_2 (cast `/Game/Blueprints/Player/Player_BP` (`GameplayStatics.GetPlayerCharacter` 0)))
        (bind _output_get_2 (set `/Game/Blueprints/Player/Player_BP.isReloading` true _asplayer_bp_2))))
    (return _output_get _output_get_2)))

(fn `UserConstructionScript`)